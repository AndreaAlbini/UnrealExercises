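; BP_Turret is a player-operated turret with single, burst and automatic fire modes.
; Overlapping its Box enables player input and adds the IMC_Turret mapping context, with both undone on leaving.
; Enhanced Input actions yaw the Cube or spawn BP_FirstPersonProjectile at ShotPoint.
; Burst fire uses a counted Delay loop, while automatic fire toggles via a FlipFlop feeding the looping AutomaticShot event.
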(event `self.Box.OnComponentBeginOverlap`
  (params (OverlappedComponent :type "PrimitiveComponent Object Reference") (OtherActor :type "Actor Object Reference") (OtherComp :type "PrimitiveComponent Object Reference") (OtherBodyIndex :type Integer) (bFromSweep :type Boolean) (SweepResult :type "HitResult Structure (by ref)"))
  (bind _returnvalue (`GameplayStatics.GetPlayerController` 0))
  (if (== OtherActor (`GameplayStatics.GetPlayerCharacter` 0))
    (`self.EnableInput` _returnvalue)
    (`KismetSystemLibrary.Delay` 0.2)
    (message `EnhancedInputSubsystemInterface.AddMappingContext` (pcsubsystem `EnhancedInputLocalPlayerSubsystem` _returnvalue) "/Game/MyFP/Turret/Input/IMC_Turret.IMC_Turret" 0 (struct))))

(event `self.Box.OnComponentEndOverlap`
  (params (OverlappedComponent :type "PrimitiveComponent Object Reference") (OtherActor :type "Actor Object Reference") (OtherComp :type "PrimitiveComponent Object Reference") (OtherBodyIndex :type Integer))
  (bind _returnvalue (`GameplayStatics.GetPlayerController` 0))
  (if (== OtherActor (`GameplayStatics.GetPlayerCharacter` 0))
    (`self.DisableInput` _returnvalue)
    (`KismetSystemLibrary.Delay` 0.2)
    (message `EnhancedInputSubsystemInterface.RemoveMappingContext` (pcsubsystem `EnhancedInputLocalPlayerSubsystem` _returnvalue) null (struct))))

(event `EnhancedInput|/Game/MyFP/Turret/Input/Action/IA_SingleShot`
  (params (ActionValue :type Boolean) (ElapsedSeconds :type "Float (double-precision)") (TriggeredSeconds :type "Float (double-precision)") (InputAction :type "InputAction Object Reference" :default "/Game/MyFP/Turret/Input/Action/IA_SingleShot.IA_SingleShot"))
  (:`Started`
    (`|SpawnActorFromClass` "/Game/FirstPerson/Blueprints/BP_FirstPersonProjectile.BP_FirstPersonProjectile_C" (`SceneComponent.K2_GetComponentToWorld` (`self.ShotPoint`)) "Undefined" "MultiplyWithRoot" null null)))

(event `EnhancedInput|/Game/MyFP/Turret/Input/Action/IA_SemiAutomaticShot`
  (params (ActionValue :type Boolean) (ElapsedSeconds :type "Float (double-precision)") (TriggeredSeconds :type "Float (double-precision)") (InputAction :type "InputAction Object Reference" :default "/Game/MyFP/Turret/Input/Action/IA_SemiAutomaticShot.IA_SemiAutomaticShot"))
  (:`Started`
    (if (< (`self.Instantiated projectiles`) (`self.ProjectilesNumber`)) :!label _label
      (`|SpawnActorFromClass` "/Game/FirstPerson/Blueprints/BP_FirstPersonProjectile.BP_FirstPersonProjectile_C" (`SceneComponent.K2_GetComponentToWorld` (`self.ShotPoint`)) "Undefined" "MultiplyWithRoot" null null)
      (`KismetSystemLibrary.Delay` (`self.ProjectilesDelay`))
      (`/Engine/EditorBlueprintResources/StandardMacros.IncrementInt` (`self.Instantiated projectiles`)
        (:`  `
          (goto _label)))
      (else
        (set `self.Instantiated projectiles` 0)))))

(event `EnhancedInput|/Game/MyFP/Turret/Input/Action/IA_AutomaticShot`
  (params (ActionValue :type Boolean) (ElapsedSeconds :type "Float (double-precision)") (TriggeredSeconds :type "Float (double-precision)") (InputAction :type "InputAction Object Reference" :default "/Game/MyFP/Turret/Input/Action/IA_AutomaticShot.IA_AutomaticShot"))
  (:`Started`
    (bind _isa (`/Engine/EditorBlueprintResources/StandardMacros.FlipFlop`)
      (:`A`
        _)
      (:`B`
        _))
    (`self.AutomaticShot` _isa)))

(event `EnhancedInput|/Game/MyFP/Turret/Input/Action/IA_RotateTurret`
  (params (ActionValue :type "Float (double-precision)") (ElapsedSeconds :type "Float (double-precision)") (TriggeredSeconds :type "Float (double-precision)") (InputAction :type "InputAction Object Reference" :default "/Game/MyFP/Turret/Input/Action/IA_RotateTurret.IA_RotateTurret"))
  (:`Triggered`
    (`SceneComponent.K2_AddRelativeRotation` (`self.Cube`) (`KismetMathLibrary.MakeRotator` 0.0 0.0 ActionValue) false false)))

(event `AutomaticShot`
  (params (Condition :type Boolean))
  (if Condition :!label _label_2
    (`|SpawnActorFromClass` "/Game/FirstPerson/Blueprints/BP_FirstPersonProjectile.BP_FirstPersonProjectile_C" (`SceneComponent.K2_GetComponentToWorld` (`self.ShotPoint`)) "Undefined" "MultiplyWithRoot" null null)
    (`KismetSystemLibrary.Delay` (`self.ProjectilesDelay`))
    (goto _label_2)))

(fn `UserConstructionScript`)
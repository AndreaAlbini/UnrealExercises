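; BP_Rifle is a pickup weapon for BP_MyFPC that fires normal and charged shots and can be dropped.
; Sphere overlap attaches it to the first-person mesh's GripPoint, sets HasRifle, enables input and, after a delay, adds IMC_Gun.
; Charging grows a sphere; completion spawns BP_BigProjectile and hides it, while cancellation shrinks it away through a Timeline.
; Dropping detaches the rifle, clears HasRifle and removes the mapping context.
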(event `self.SphereCollision.OnComponentBeginOverlap`
  (params (OverlappedComponent :type "PrimitiveComponent Object Reference") (OtherActor :type "Actor Object Reference") (OtherComp :type "PrimitiveComponent Object Reference") (OtherBodyIndex :type Integer) (bFromSweep :type Boolean) (SweepResult :type "HitResult Structure (by ref)"))
  (bind _returnvalue (`GameplayStatics.GetPlayerController` 0))
  (bind _asbp_my_fpc (cast `/Game/MyFP/Player/BP_MyFPC` OtherActor))
  (set `/Game/MyFP/Player/BP_MyFPC.bHasRifle` true _asbp_my_fpc)
  (bind _output_get (set `self.As BP My FPC` _asbp_my_fpc))
  (`self.K2_AttachToComponent` (`/Game/MyFP/Player/BP_MyFPC.FirstPersonMesh` _output_get) "GripPoint" "SnapToTarget" "SnapToTarget" "SnapToTarget")
  (`self.EnableInput` _returnvalue)
  (`KismetSystemLibrary.Delay` 0.2)
  (`EnhancedInputSubsystemInterface.AddMappingContext` (pcsubsystem `EnhancedInputLocalPlayerSubsystem` _returnvalue) "/Game/MyFP/Rifle/Input/IMC_Gun.IMC_Gun" 0 (struct)))

(event `EnhancedInput|/Game/MyFP/Rifle/Input/Action/IA_GunShot`
  (params (ActionValue :type Boolean) (ElapsedSeconds :type "Float (double-precision)") (TriggeredSeconds :type "Float (double-precision)") (InputAction :type "InputAction Object Reference" :default "/Game/MyFP/Rifle/Input/Action/IA_GunShot.IA_GunShot"))
  (:`Started`
    (`|SpawnActorFromClass` "/Game/FirstPerson/Blueprints/BP_FirstPersonProjectile.BP_FirstPersonProjectile_C" (`SceneComponent.K2_GetComponentToWorld` (`self.SpawnPoint`)) "Undefined" "MultiplyWithRoot" null null)))

(event `EnhancedInput|/Game/MyFP/Rifle/Input/Action/IA_Drop`
  (params (ActionValue :type Boolean) (ElapsedSeconds :type "Float (double-precision)") (TriggeredSeconds :type "Float (double-precision)") (InputAction :type "InputAction Object Reference" :default "/Game/MyFP/Rifle/Input/Action/IA_Drop.IA_Drop"))
  (:`Started`
    (`self.K2_DetachFromActor` "KeepWorld" "KeepWorld" "KeepWorld")
    (set `/Game/MyFP/Player/BP_MyFPC.bHasRifle` false (`self.As BP My FPC`))
    (message `EnhancedInputSubsystemInterface.RemoveMappingContext` (pcsubsystem `EnhancedInputLocalPlayerSubsystem` (`GameplayStatics.GetPlayerController` 0)) "/Game/MyFP/Rifle/Input/IMC_Gun.IMC_Gun" (struct))))

(event `EnhancedInput|/Game/MyFP/Rifle/Input/Action/IA_ChargedShot`
  (params (ActionValue :type Boolean) (ElapsedSeconds :type "Float (double-precision)") (TriggeredSeconds :type "Float (double-precision)") (InputAction :type "InputAction Object Reference" :default "/Game/MyFP/Rifle/Input/Action/IA_ChargedShot.IA_ChargedShot"))
  (bind _sphere (`self.Sphere`))
  (:`Started`
    (`SceneComponent.SetRelativeScale3D` _sphere (0.0 0.0 0.0))
    (`SceneComponent.SetVisibility` _sphere true false))
  (:`Ongoing`
    (`SceneComponent.SetRelativeScale3D` _sphere (`KismetMathLibrary.Conv_DoubleToVector` (`KismetMathLibrary.FMin` (`KismetMathLibrary.Lerp` 0.0 0.7 ElapsedSeconds) 0.7))))
  (:`Canceled`
    (set `self.ElapsedSeconds` ElapsedSeconds)
    (bind (_direction _newtrack_0) (`Timeline|Timeline` :!via `PlayFromStart`)
      (:`Update`
        (`SceneComponent.SetRelativeScale3D` _sphere (`KismetMathLibrary.Conv_DoubleToVector` (`KismetMathLibrary.Lerp` (`KismetMathLibrary.FMin` (`self.ElapsedSeconds`) 0.7) 0.0 _newtrack_0))))
      (:`Finished`
        (`SceneComponent.SetVisibility` _sphere false false :!label _label))))
  (:`Completed`
    (`|SpawnActorFromClass` "/Game/MyFP/Rifle/BP_BigProjectile.BP_BigProjectile_C" (`SceneComponent.K2_GetComponentToWorld` (`self.SpawnPoint`)) "Undefined" "MultiplyWithRoot" null null)
    (goto _label)))

(fn `UserConstructionScript`)
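; Seesaw actor that pitches around its Pivot component while the player character is inside its Box trigger.
; Box overlaps toggle CanRotate, which Tick passes to the Rotation event.
; Rotation picks the tilt direction by comparing 2D distances from Side to Pivot and to the player's mesh.
; The per-frame pitch step grows with the player's distance from Pivot; MinRotation and MaxRotation clamp that step, without delta-time scaling.
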(event `self.Box.OnComponentBeginOverlap`
  (params (OverlappedComponent :type "PrimitiveComponent Object Reference") (OtherActor :type "Actor Object Reference") (OtherComp :type "PrimitiveComponent Object Reference") (OtherBodyIndex :type Integer) (bFromSweep :type Boolean) (SweepResult :type "HitResult Structure (by ref)"))
  (if (== OtherActor (`GameplayStatics.GetPlayerCharacter` 0))
    (set `self.CanRotate` true)))

(event `self.Box.OnComponentEndOverlap`
  (params (OverlappedComponent :type "PrimitiveComponent Object Reference") (OtherActor :type "Actor Object Reference") (OtherComp :type "PrimitiveComponent Object Reference") (OtherBodyIndex :type Integer))
  (if (== OtherActor (`GameplayStatics.GetPlayerCharacter` 0))
    (set `self.CanRotate` false)))

(event `self.ReceiveTick`
  (params (DeltaSeconds :type "Float (single-precision)"))
  (`self.Rotation` (`self.CanRotate`)))

(event `Rotation`
  (params (Condition :type Boolean))
  (bind _returnvalue (`SceneComponent.K2_GetComponentLocation` (`self.Side`)))
  (bind _returnvalue_2 (`SceneComponent.K2_GetComponentLocation` (`self.Pivot`)))
  (bind _returnvalue_3 (`SceneComponent.K2_GetComponentLocation` (`Character.Mesh` (`GameplayStatics.GetPlayerCharacter` 0))))
  (if Condition
    (if (>= (`KismetMathLibrary.Vector_Distance2D` _returnvalue _returnvalue_2) (`KismetMathLibrary.Vector_Distance2D` _returnvalue _returnvalue_3))
      (set `self.VersoDiRotazione` 1.0)
      (else
        (set `self.VersoDiRotazione` -1.0)))
    (`SceneComponent.K2_AddLocalRotation` (`self.Pivot`) (`KismetMathLibrary.MakeRotator` 0.0 (`KismetMathLibrary.FClamp` (* (/ (`KismetMathLibrary.Vector_Distance2D` _returnvalue_2 _returnvalue_3) 100.0) (`self.VersoDiRotazione`)) (`self.MinRotation`) (`self.MaxRotation`))) false false)))

(fn `UserConstructionScript`)
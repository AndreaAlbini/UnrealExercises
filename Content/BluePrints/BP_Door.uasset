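; BP_Door is a proximity door that swings open around the player and displays a text prompt.
; When player character 0 enters the Box, the TextRender switches to the trigger text and the DoorOpen timeline yaws the Scene component by a configurable angle.
; On exit, checked by the "Player" actor tag rather than character identity, the start text returns and the timeline reverses after a configurable delay.
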(event `self.ReceiveBeginPlay`
  (`TextRenderComponent.K2_SetText` (`self.TextRender`) (`self.StartText`)))

(event `self.Box.OnComponentBeginOverlap`
  (params (OverlappedComponent :type "PrimitiveComponent Object Reference") (OtherActor :type "Actor Object Reference") (OtherComp :type "PrimitiveComponent Object Reference") (OtherBodyIndex :type Integer) (bFromSweep :type Boolean) (SweepResult :type "HitResult Structure (by ref)"))
  (if (== OtherActor (`GameplayStatics.GetPlayerCharacter` 0))
    (`TextRenderComponent.K2_SetText` (`self.TextRender`) (`self.TriggerText`))
    (bind (_direction _newtrack_0) (`Timeline|DoorOpen` :!label _label)
      (:`Update`
        (`SceneComponent.K2_SetRelativeRotation` (`self.Scene`) (`KismetMathLibrary.MakeRotator` 0.0 0.0 (* _newtrack_0 (`self.Angle`))) false false)))))

(event `self.Box.OnComponentEndOverlap`
  (params (OverlappedComponent :type "PrimitiveComponent Object Reference") (OtherActor :type "Actor Object Reference") (OtherComp :type "PrimitiveComponent Object Reference") (OtherBodyIndex :type Integer))
  (if (`self.ActorHasTag` OtherActor "Player")
    (`TextRenderComponent.K2_SetText` (`self.TextRender`) (`self.StartText`))
    (`KismetSystemLibrary.Delay` (`self.CloseDelay`))
    (goto _label :!via `Reverse`)))

(fn `UserConstructionScript`)
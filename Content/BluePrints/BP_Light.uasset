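; BP_Light is a proximity-activated spotlight that brightens as the player approaches.
; On BeginPlay it starts hidden at MinIntensity.
; Each Tick shows it within AccensionDistance of the player horizontally and maps that distance to intensity up to MaxIntensity, using MinIntensity as a distance bound.
; The box overlap events are empty, leaving a tag-filtered Timeline fade disconnected.
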(event `self.ReceiveBeginPlay`
  (bind _spotlight (`self.SpotLight`))
  (`LightComponent.SetIntensity` _spotlight (`self.MinIntensity`))
  (`SceneComponent.SetVisibility` _spotlight false false))

(event `self.Box.OnComponentBeginOverlap`
  (params (OverlappedComponent :type "PrimitiveComponent Object Reference") (OtherActor :type "Actor Object Reference") (OtherComp :type "PrimitiveComponent Object Reference") (OtherBodyIndex :type Integer) (bFromSweep :type Boolean) (SweepResult :type "HitResult Structure (by ref)")))

(event `self.Box.OnComponentEndOverlap`
  (params (OverlappedComponent :type "PrimitiveComponent Object Reference") (OtherActor :type "Actor Object Reference") (OtherComp :type "PrimitiveComponent Object Reference") (OtherBodyIndex :type Integer)))

(event `self.ReceiveTick`
  (params (DeltaSeconds :type "Float (single-precision)"))
  (bind _accensiondistance (`self.AccensionDistance`))
  (bind _returnvalue (`self.GetHorizontalDistanceTo` (`GameplayStatics.GetPlayerCharacter` 0)))
  (`SceneComponent.SetVisibility` (`self.SpotLight`) (<= _returnvalue _accensiondistance) false)
  (`LightComponent.SetIntensity` (`self.SpotLight`) (`KismetMathLibrary.MapRangeClamped` _returnvalue _accensiondistance (`self.MinIntensity`) 0.0 (`self.MaxIntensity`))))

(fn `UserConstructionScript`)
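; BP_Baloon is an inflatable balloon actor that grows when pumped, changes color by size and eventually explodes by being destroyed.
; Pump takes a condition that either starts or stops a Timeline, which adds to the sphere's scale each update and replays until the red threshold.
; A dynamic material turns green, orange, then red at size thresholds.
; At red, a delay precedes destruction if the pump condition still holds.
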(event `self.ReceiveBeginPlay`
  (bind _returnvalue (`PrimitiveComponent.CreateDynamicMaterialInstance` (`self.Sphere`) 0 "/Game/BluePrints/M_Baloon.M_Baloon" "None"))
  (set `self.Material` _returnvalue))

(event `Pump`
  (params (Condition :type Boolean))
  (bind _material (`self.Material`))
  (bind _sphere (`self.Sphere`))
  (bind _relativescale3d_x (`KismetMathLibrary.BreakVector` (`SceneComponent.RelativeScale3D` (`self.Sphere`))))
  (if Condition :!label _label
    (bind (_direction _enlargementrate) (`Timeline|Timeline` :!via `PlayFromStart` :!label _label_2)
      (:`Update`
        (`SceneComponent.SetRelativeScale3D` _sphere (+ (* (`self.EnlargementRate`) _enlargementrate) (`SceneComponent.RelativeScale3D` _sphere)))
        (if (>= _relativescale3d_x (`self.GreenSizeThreshold`))
          (`MaterialInstanceDynamic.SetVectorParameterValue` _material "Color" (struct :`G` 1.0 :`A` 1.0))
          (if (>= _relativescale3d_x (`self.OrangeSizeThreshold`))
            (`MaterialInstanceDynamic.SetVectorParameterValue` _material "Color" (struct :`R` 1.0 :`G` 0.147163 :`A` 1.0)))))
      (:`Finished`
        (if (< _relativescale3d_x (`self.RedSizeThreshold`))
          (goto _label)
          (else
            (`MaterialInstanceDynamic.SetVectorParameterValue` (`self.Material`) "Color" (struct :`R` 1.0 :`A` 1.0))
            (`KismetSystemLibrary.Delay` (`self.ExplosionTimer`))
            (if Condition
              (`self.K2_DestroyActor`))))))
    (else
      (goto _label_2 :!via `Stop`))))

(fn `UserConstructionScript`)
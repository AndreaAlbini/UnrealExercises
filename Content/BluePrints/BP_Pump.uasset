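; BP_Pump is an interactable pump that lets the player pump a balloon by holding C while standing nearby.
; A Box overlap enables the actor's input when the player character enters and disables it on exit.
; Pressing and releasing C finds a BP_Baloon through GetActorOfClass and calls its Pump function with true or false.
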(event `Key|C`
  (params (Key :type "Key Structure"))
  (:`Pressed`
    (bind _returnvalue (`GameplayStatics.GetActorOfClass` "/Game/BluePrints/BP_Baloon.BP_Baloon_C"))
    (`/Game/BluePrints/BP_Baloon.Pump` _returnvalue true))
  (:`Released`
    (bind _returnvalue_2 (`GameplayStatics.GetActorOfClass` "/Game/BluePrints/BP_Baloon.BP_Baloon_C"))
    (`/Game/BluePrints/BP_Baloon.Pump` _returnvalue_2 false)))

(event `self.Box.OnComponentBeginOverlap`
  (params (OverlappedComponent :type "PrimitiveComponent Object Reference") (OtherActor :type "Actor Object Reference") (OtherComp :type "PrimitiveComponent Object Reference") (OtherBodyIndex :type Integer) (bFromSweep :type Boolean) (SweepResult :type "HitResult Structure (by ref)"))
  (if (== OtherActor (`GameplayStatics.GetPlayerCharacter` 0))
    (`self.EnableInput` (`GameplayStatics.GetPlayerController` 0))))

(event `self.Box.OnComponentEndOverlap`
  (params (OverlappedComponent :type "PrimitiveComponent Object Reference") (OtherActor :type "Actor Object Reference") (OtherComp :type "PrimitiveComponent Object Reference") (OtherBodyIndex :type Integer))
  (if (== OtherActor (`GameplayStatics.GetPlayerCharacter` 0))
    (`self.DisableInput` (`GameplayStatics.GetPlayerController` 0))))

(fn `UserConstructionScript`)
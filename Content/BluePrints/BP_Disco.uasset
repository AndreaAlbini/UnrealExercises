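; BP_Disco is a disco sphere that flashes random colors once the player enters its box trigger.
; BeginPlay creates a dynamic M_Disco material on the sphere for runtime color and brightness changes.
; The Disco event re-arms its own timer with a random interval, setting a random color and the emissive brightness.
; Leaving the box never clears the timer and writes white to an unnamed parameter, so flashing continues.
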(event `self.ReceiveBeginPlay`
  (bind _returnvalue (`PrimitiveComponent.CreateDynamicMaterialInstance` (`self.Sphere`) 0 "/Game/BluePrints/M_Disco.M_Disco" "None"))
  (set `self.MaterialRef` _returnvalue))

(event `self.Box.OnComponentBeginOverlap`
  (params (OverlappedComponent :type "PrimitiveComponent Object Reference") (OtherActor :type "Actor Object Reference") (OtherComp :type "PrimitiveComponent Object Reference") (OtherBodyIndex :type Integer) (bFromSweep :type Boolean) (SweepResult :type "HitResult Structure (by ref)"))
  (if (== OtherActor (`GameplayStatics.GetPlayerCharacter` 0))
    (`self.Disco`)))

(event `Disco`
  (bind _materialref (`self.MaterialRef`))
  (`KismetSystemLibrary.K2_SetTimerDelegate` (delegate `Disco`) (`KismetMathLibrary.RandomFloatInRange` (`self.MinTime`) (`self.MaxTime`)) true)
  (`MaterialInstanceDynamic.SetVectorParameterValue` _materialref "Color" (`KismetArrayLibrary.Array_Random` (`self.Color`)))
  (`MaterialInstanceDynamic.SetScalarParameterValue` _materialref "Brightness" (`self.Emissivity`)))

(event `self.Box.OnComponentEndOverlap`
  (params (OverlappedComponent :type "PrimitiveComponent Object Reference") (OtherActor :type "Actor Object Reference") (OtherComp :type "PrimitiveComponent Object Reference") (OtherBodyIndex :type Integer))
  (if (== OtherActor (`GameplayStatics.GetPlayerCharacter` 0))
    (`MaterialInstanceDynamic.SetVectorParameterValue` (`self.MaterialRef`) "None" (struct :`R` 1.0 :`G` 1.0 :`B` 1.0 :`A` 1.0))))

(fn `UserConstructionScript`)
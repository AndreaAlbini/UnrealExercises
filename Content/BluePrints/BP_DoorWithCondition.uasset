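; Door actor that slides its Cube along Z when OpenDoor is called, with unfinished key and coin conditions.
; OpenDoor plays a Timeline that scales the Movement offset on top of a fixed base height.
; The HasKey check and the coin-threshold check with its TextRender counter are disconnected and never run.
; The Box overlap only casts to BP_ThirdPersonCharacter, so it does not open the door.
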(event `self.Box.OnComponentBeginOverlap`
  (params (OverlappedComponent :type "PrimitiveComponent Object Reference") (OtherActor :type "Actor Object Reference") (OtherComp :type "PrimitiveComponent Object Reference") (OtherBodyIndex :type Integer) (bFromSweep :type Boolean) (SweepResult :type "HitResult Structure (by ref)"))
  (cast `/Game/ThirdPerson/Blueprints/BP_ThirdPersonCharacter` OtherActor))

(event `OpenDoor`
  ;[1 1 1] OpenDoor
  (bind (_direction _newtrack_0) (`Timeline|Timeline`)
    (:`Update`
      (`SceneComponent.K2_SetRelativeLocation` (`self.Cube`) (`KismetMathLibrary.MakeVector` 0.0 0.0 (+ (* _newtrack_0 (`self.movement`)) 100.0)) false false))))

(fn `UserConstructionScript`)
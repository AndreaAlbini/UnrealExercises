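; Moving platform Blueprint that shuttles its Cube back and forth between Point1 and Point2, starting at BeginPlay.
; A Timeline track drives a lerp between the two points' relative locations, setting the Cube's position without sweeping.
; When the Timeline finishes, it waits for PlatformPause, then a FlipFlop alternates between playing from start and reversing, looping indefinitely.
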(event `self.ReceiveBeginPlay`
  (`self.MovePlatform`))

(event `MovePlatform`
  (`/Engine/EditorBlueprintResources/StandardMacros.FlipFlop` :!label _label
    (:`A`
      (bind (_direction _newtrack_0) (`Timeline|Timeline` :!via `PlayFromStart` :!label _label_2)
        (:`Update`
          (`SceneComponent.K2_SetRelativeLocation` (`self.Cube`) (`KismetMathLibrary.VLerp` (`SceneComponent.RelativeLocation` (`self.Point1`)) (`SceneComponent.RelativeLocation` (`self.Point2`)) _newtrack_0) false false))
        (:`Finished`
          (`KismetSystemLibrary.Delay` (`self.PlatformPause`))
          (goto _label))))
    (:`B`
      (goto _label_2 :!via `Reverse`))))

(fn `UserConstructionScript`)
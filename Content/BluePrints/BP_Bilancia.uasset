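; BP_Bilancia is a weighing scale that shows the total mass of objects inside its box trigger on a text render in kilograms.
; Overlap begin and end events on the box add or subtract the overlapping component's mass from a running TotalMass.
; Each change immediately rewrites the displayed text, so the readout is event-driven and uses no tick.
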(event `self.Box.OnComponentBeginOverlap`
  (params (OverlappedComponent :type "PrimitiveComponent Object Reference") (OtherActor :type "Actor Object Reference") (OtherComp :type "PrimitiveComponent Object Reference") (OtherBodyIndex :type Integer) (bFromSweep :type Boolean) (SweepResult :type "HitResult Structure (by ref)"))
  (bind _output_get (set `self.TotalMass` (+ (`PrimitiveComponent.GetMass` OtherComp) (`self.TotalMass`))))
  (`TextRenderComponent.K2_SetText` (`self.TextRender`) (`|FormatText` "{TotalMass} Kg" _output_get)))

(event `self.Box.OnComponentEndOverlap`
  (params (OverlappedComponent :type "PrimitiveComponent Object Reference") (OtherActor :type "Actor Object Reference") (OtherComp :type "PrimitiveComponent Object Reference") (OtherBodyIndex :type Integer))
  (bind _output_get (set `self.TotalMass` (- (`self.TotalMass`) (`PrimitiveComponent.GetMass` OtherComp))))
  (`TextRenderComponent.K2_SetText` (`self.TextRender`) (`|FormatText` "{TotalMass} Kg" _output_get)))

(fn `UserConstructionScript`)
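; Actor Blueprint that spins a cube and animates the color of a spot light.
; BeginPlay triggers a CubeRotation event that plays a timeline.
; Each timeline update adds local rotation to the cube, scaling RotationSpeed by the Rotation track, and applies the LightColor track to the spot light.
; An alternative Tick-based rotation remains in the graph but is disconnected.
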(event `self.ReceiveBeginPlay`
  (`self.CubeRotation`))

(event `CubeRotation`
  (bind (_rotation_speed_x _rotation_speed_y _rotation_speed_z) (`KismetMathLibrary.BreakVector` (`self.Rotation Speed`)))
  (bind (_direction _rotation _lightcolor) (`Timeline|Timeline`)
    (:`Update`
      (`SceneComponent.K2_AddLocalRotation` (`self.Cube`) (`KismetMathLibrary.MakeRotator` (* _rotation_speed_x _rotation) (* _rotation_speed_y _rotation) (* _rotation_speed_z _rotation)) false false)
      (`LightComponent.SetLightColor` (`self.SpotLight`) _lightcolor true))))

(event `self.ReceiveTick`
  (params (DeltaSeconds :type "Float (single-precision)"))
  ;[1 1 1] Rotation with Tick
)

(fn `UserConstructionScript`)
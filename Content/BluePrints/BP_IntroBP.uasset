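; BP_IntroBP is an actor that bobs two cube components vertically in opposite directions.
; BeginPlay caches each cube's relative start location.
; Every Tick, a sine of game time times Speed is remapped to 0–1 and scaled by Ampiezza (amplitude), so Cube oscillates upward from its start and Cube1 mirrors it downward.
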(event `self.ReceiveBeginPlay`
  (set `self.StartPositionCube` (`SceneComponent.RelativeLocation` (`self.Cube`)))
  (set `self.StartPositionCube1` (`SceneComponent.RelativeLocation` (`self.Cube1`))))

(event `self.ReceiveTick`
  (params (DeltaSeconds :type "Float (single-precision)"))
  (bind (_startpositioncube1_x _startpositioncube1_y _startpositioncube1_z) (`KismetMathLibrary.BreakVector` (`self.StartPositionCube1`)))
  (bind (_startpositioncube_x _startpositioncube_y _startpositioncube_z) (`KismetMathLibrary.BreakVector` (`self.StartPositionCube`)))
  (bind _returnvalue (* (`KismetMathLibrary.MapRangeClamped` (`KismetMathLibrary.Sin` (* (`GameplayStatics.GetTimeSeconds`) (`self.Speed`))) -1.0 1.0 0.0 1.0) (`self.Ampiezza`)))
  ;[1 1 1] CubeMovement
  (`SceneComponent.K2_SetRelativeLocation` (`self.Cube`) (`KismetMathLibrary.MakeVector` _startpositioncube_x _startpositioncube_y (+ _startpositioncube_z _returnvalue)) false false)
  (`SceneComponent.K2_SetRelativeLocation` (`self.Cube1`) (`KismetMathLibrary.MakeVector` _startpositioncube1_x _startpositioncube1_y (+ _startpositioncube1_z (* _returnvalue -1.0))) false false))

(fn `UserConstructionScript`)
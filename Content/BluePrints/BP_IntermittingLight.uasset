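; BP_IntermittingLight is a spot light Blueprint that blinks on and off at random intervals while changing color.
; BeginPlay calls the Light event, which re-arms a timer on itself with a new random delay between MinTime and MaxTime on each call.
; Each call toggles the SpotLight's visibility through a FlipFlop and sets its color to a random entry from the NewLightColor array.
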(event `self.ReceiveBeginPlay`
  (`self.Light`))

(event `Light`
  (bind _spotlight (`self.SpotLight`))
  (`KismetSystemLibrary.K2_SetTimerDelegate` (delegate `Light`) (`KismetMathLibrary.RandomFloatInRange` (`self.MinTime`) (`self.MaxTime`)) true)
  (bind _isa (`/Engine/EditorBlueprintResources/StandardMacros.FlipFlop`)
    (:`A`
      _)
    (:`B`
      _))
  (`SceneComponent.SetVisibility` _spotlight _isa false)
  (`LightComponent.SetLightColor` _spotlight (`KismetArrayLibrary.Array_Random` (`self.New Light Color`)) false))

(fn `UserConstructionScript`)
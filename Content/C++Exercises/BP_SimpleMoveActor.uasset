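; BP_SimpleMoveActor is a C++ exercise actor that gives a random-outcome reaction to its KillEverythingwithGiantMassiveExplosion event.
; The event prints RandomProbability, then branches on its value: low does nothing, middle spawns a Niagara system at the Cube's location, high destroys the actor.
; The graph only reads that value and contains no movement logic, with BeginPlay, overlap, Tick and construction left empty.
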(event `self.KillEverythingWithGiantMassiveExplosion`
  (bind _randomprobability (`self.RandomProbability`))
  (`KismetSystemLibrary.PrintString` (`KismetStringLibrary.Conv_IntToString` _randomprobability))
  (if (< _randomprobability 6)
    _
    (elif (< _randomprobability 9)
      (`NiagaraFunctionLibrary.SpawnSystemAtLocation` "/Game/C++Exercises/NewNiagaraSystem.NewNiagaraSystem" (`SceneComponent.K2_GetComponentLocation` (`self.Cube`)))
      (else
        (`self.K2_DestroyActor`)))))

(fn `UserConstructionScript`)